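; Poliduende policeman enemy character, a flipbook sprite that continually turns to face the first-person player, chases and shoots.
; A state enum selects the flipbook and gates a delay-based firing loop that spawns projectiles while the player is detected.
; When the player leaves the detection volume, it pauses, then runs after them with AI MoveTo.
; Tagged player projectiles flash it red: head hits kill instantly, body hits decrement HP and interrupt shooting.
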(event OnComponentBeginOverlap(HeadCollider)
  (params (OverlappedComponent :type Primitive%20Component%20Object%20Reference) (OtherActor :type Actor%20Object%20Reference) (OtherComp :type Primitive%20Component%20Object%20Reference) (OtherBodyIndex :type Integer) (bFromSweep :type Boolean) (SweepResult :type Hit%20Result%20Structure%20%28by%20ref%29))
  (if (Actor|ActorHasTag OtherActor "PlayerProjectil")
    (CallFunction|PolicemanReceiveDamage true)))

(event OnComponentBeginOverlap(CapsuleComponent)
  (params (OverlappedComponent :type Primitive%20Component%20Object%20Reference) (OtherActor :type Actor%20Object%20Reference) (OtherComp :type Primitive%20Component%20Object%20Reference) (OtherBodyIndex :type Integer) (bFromSweep :type Boolean) (SweepResult :type Hit%20Result%20Structure%20%28by%20ref%29))
  (if (Actor|ActorHasTag OtherActor "PlayerProjectil")
    (CallFunction|SetPolicemanStates "NewEnumerator3")
    (CallFunction|PolicemanReceiveDamage false)
    (Utilities|FlowControl|Delay 1.0)
    (if (Collision|IsOverlappingActor (Variables|Default|GetPlayerDetection) (.AsFirst%20Person%20Character (Utilities|Casting|CastToFirstPersonCharacter (Game|Player|GetPlayerPawn 0))) :!class /Script/Engine.PrimitiveComponent)
      (CallFunction|PlayerDetected)
      (else
        (CallFunction|RuntoPlayer)))))

(event OnComponentBeginOverlap(PlayerDetection)
  (params (OverlappedComponent :type Primitive%20Component%20Object%20Reference) (OtherActor :type Actor%20Object%20Reference) (OtherComp :type Primitive%20Component%20Object%20Reference) (OtherBodyIndex :type Integer) (bFromSweep :type Boolean) (SweepResult :type Hit%20Result%20Structure%20%28by%20ref%29))
  (if (Components|ComponentHasTag OtherComp "PlayerCollider")
    (switch Utilities|FlowControl|Switch|SwitchonPoliduendeStates_List (Variables|Default|GetPoliceStates)
      (:NewEnumerator0
        _)
      (:NewEnumerator5
        _))
    (CallFunction|PlayerDetected)))

(event OnComponentEndOverlap(PlayerDetection)
  (params (OverlappedComponent :type Primitive%20Component%20Object%20Reference) (OtherActor :type Actor%20Object%20Reference) (OtherComp :type Primitive%20Component%20Object%20Reference) (OtherBodyIndex :type Integer))
  (bind _returnvalue (Game|Player|GetPlayerPawn 0))
  (bind _asfirst_person_character (Utilities|Casting|CastToFirstPersonCharacter _returnvalue))
  (if (Components|ComponentHasTag OtherComp "PlayerCollider")
    (CallFunction|SetPolicemanStates "NewEnumerator0")
    (Utilities|FlowControl|Delay 2.0)
    (if (Collision|IsOverlappingActor (Variables|Default|GetPlayerDetection) (.AsFirst%20Person%20Character (Utilities|Casting|CastToFirstPersonCharacter (Game|Player|GetPlayerPawn 0))) :!class /Script/Engine.PrimitiveComponent)
      (CallFunction|PlayerDetected)
      (else
        (CallFunction|SetPolicemanStates "NewEnumerator5")
        (AI|AIMoveTo self (Transformation|GetWorldLocation (Variables|/Script/Engine.Character|GetCapsuleComponent _asfirst_person_character)) _asfirst_person_character 5.0 true)))))

(event Custom|LookToPlayer
  (Transformation|SetActorRotation (Math|Rotator|MakeRotator 0.0 0.0 (.yaw (Math|Interpolation|RInterpTo (Transformation|GetActorRotation) (Math|Rotator|FindLookatRotation (Transformation|GetActorLocation) (Transformation|GetActorLocation (Variables|Default|GetChar_Reff))) (Utilities|Time|GetWorldDeltaSeconds) 0.0))))
  (Utilities|FlowControl|Delay 0.01)
  (CallFunction|LooktoPlayer))

(event Custom|PolicemanReceiveDamage
  (params (Headshoot? :type Boolean))
  (Components|Movement|StopMovementImmediately (Variables|Character|GetCharacterMovement))
  (Utilities|FlowControl|Sequence
    (:then_0
      (if Headshoot?
        (Variables|Default|SetPoliceman_HP 0)
        (Components|DestroyComponent (Variables|Default|GetHeadCollider))
        (Utilities|FlowControl|Delay 0.2 :!label _label)
        (Actor|DestroyActor)
        (else
          (bind _result (Math|Integer|DecrementInt (Variables|Default|GetPoliceman_HP))
            (:%20%20
              (if (<= _result 0)
                (goto _label)))))))
    (:then_1
      (Sprite|SetSpriteColor (Variables|Default|GetPoliduende_FB) "(R=1.000000,G=0.000000,B=0.000000,A=1.000000)")
      (Utilities|FlowControl|Delay 0.1)
      (Sprite|SetSpriteColor (Variables|Default|GetPoliduende_FB) "(R=1.000000,G=1.000000,B=1.000000,A=1.000000)"))))

(event Custom|SetPolicemanStates
  (params (NewPoliceState :type PoliduendeStates_List%20Enum :default "NewEnumerator0"))
  (bind _output_get (Variables|Default|SetPoliceStates NewPoliceState))
  (switch Utilities|FlowControl|Switch|SwitchonPoliduendeStates_List _output_get
    (:NewEnumerator0
      (Sprite|SetFlipbook (Variables|Default|GetPoliduende_FB) "/Game/Blueprints/Art/T_Police_Idle_FB.T_Police_Idle_FB"))
    (:NewEnumerator1
      (Sprite|SetFlipbook (Variables|Default|GetPoliduende_FB) "/Game/Blueprints/Art/T_Police_Agroo_FB.T_Police_Agroo_FB"))
    (:NewEnumerator2
      (Sprite|SetFlipbook (Variables|Default|GetPoliduende_FB) "/Game/Blueprints/Art/T_Police_Shoot_FB.T_Police_Shoot_FB"))
    (:NewEnumerator3
      (Sprite|SetFlipbook (Variables|Default|GetPoliduende_FB) "/Game/Blueprints/Art/T_Police_Hit_FB.T_Police_Hit_FB"))
    (:NewEnumerator5
      (Sprite|SetFlipbook (Variables|Default|GetPoliduende_FB) "/Game/Blueprints/Art/T_Police_Run_FB.T_Police_Run_FB"))))

(event Custom|Player%20Detected
  (Components|Movement|StopMovementImmediately (Variables|Character|GetCharacterMovement self))
  (CallFunction|SetPolicemanStates "NewEnumerator1")
  (Utilities|FlowControl|Delay 1.0)
  (switch Utilities|FlowControl|Switch|SwitchonPoliduendeStates_List (Variables|Default|GetPoliceStates) :!label _label
    (:NewEnumerator1
      (CallFunction|SetPolicemanStates "NewEnumerator2")
      (Utilities|FlowControl|Delay 0.1)
      (if (Utilities|Enum|Equal(Enum) (Variables|Default|GetPoliceStates) "NewEnumerator2")
        (Game|SpawnActorfromClass "/Game/Blueprints/PoliDuende/PoliceProjectile_BP.PoliceProjectile_BP_C" (Math|Transform|MakeTransform (Transformation|GetSocketLocation (Variables|Default|GetPoliduende_FB) "BulletStart") (Transformation|GetWorldRotation (Variables|Collision|GetCapsuleComponent)) "1,1,1") "Undefined" 0 0)
        (Utilities|FlowControl|Delay 0.2)
        (CallFunction|SetPolicemanStates "NewEnumerator1")
        (Utilities|FlowControl|Delay (Math|Random|RandomFloatinRange 0.3 1.0))
        (goto _label)))))

(event Custom|RunToPlayer
  (bind _returnvalue (Game|Player|GetPlayerPawn 0))
  (bind _asfirst_person_character (Utilities|Casting|CastToFirstPersonCharacter _returnvalue))
  (CallFunction|SetPolicemanStates "NewEnumerator0")
  (Utilities|FlowControl|Delay 2.0)
  (if (Collision|IsOverlappingActor (Variables|Default|GetPlayerDetection) (.AsFirst%20Person%20Character (Utilities|Casting|CastToFirstPersonCharacter (Game|Player|GetPlayerPawn 0))) :!class /Script/Engine.PrimitiveComponent)
    (CallFunction|PlayerDetected)
    (else
      (CallFunction|SetPolicemanStates "NewEnumerator5")
      (AI|AIMoveTo self (Transformation|GetWorldLocation (Variables|/Script/Engine.Character|GetCapsuleComponent _asfirst_person_character)) _asfirst_person_character 5.0 true))))

(event EventBeginPlay
  (bind _returnvalue (Actor|GetActorOfClass "/Game/Blueprints/FirstPersonBP/Blueprints/FirstPersonCharacter.FirstPersonCharacter_C"))
  (Variables|Default|SetChar_Reff _returnvalue)
  (CallFunction|LooktoPlayer))

(fn ConstructionScript)