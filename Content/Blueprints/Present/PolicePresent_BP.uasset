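; PolicePresent_BP is a flipbook present that the player picks up through Interact unless it lies under the Christmas tree.
; At BeginPlay it checks its box for an overlapping ArbolNavidad_BP, which locks pickup and sets the sprite color to white.
; A self-calling delay loop turns it on yaw only to face the player.
; Hitting a Ground object replaces it with a fresh copy at the box transform, rerunning the tree check.
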(event OnComponentHit(Box)
  (params (HitComponent :type Primitive%20Component%20Object%20Reference) (OtherActor :type Actor%20Object%20Reference) (OtherComp :type Primitive%20Component%20Object%20Reference) (NormalImpulse :type Vector :default "0, 0, 0") (Hit :type Hit%20Result%20Structure%20%28by%20ref%29))
  (switch Utilities|FlowControl|Switch|SwitchonECollisionChannel (Collision|GetCollisionObjectType OtherComp)
    (:ECC_GameTraceChannel2
      (Game|SpawnActorfromClass "PolicePresent_BP_C" (Transformation|GetWorldTransform (Variables|Default|GetBox)) "Undefined" 0 0)
      (Actor|DestroyActor))))

(event Custom|LookToPlayer
  (Transformation|SetWorldRotation (Variables|Default|GetDefaultSceneRoot) (Math|Rotator|MakeRotator 0.0 0.0 (.yaw (Math|Interpolation|RInterpTo (Transformation|GetActorRotation) (Math|Rotator|FindLookatRotation (Transformation|GetActorLocation) (Transformation|GetActorLocation (Variables|Default|GetChar_Reff))) (Utilities|Time|GetWorldDeltaSeconds) 0.0))) false false)
  (Utilities|FlowControl|Delay 0.05)
  (CallFunction|LooktoPlayer))

(event EventBeginPlay
  (Variables|Default|SetChar_Reff (.AsFirst%20Person%20Character (Utilities|Casting|CastToFirstPersonCharacter (Game|Player|GetPlayerPawn 0))))
  (CallFunction|LooktoPlayer)
  (for _array_element (Collision|GetOverlappingActors (Variables|Default|GetBox) "/Game/Blueprints/ArbolNavidad/ArbolNavidad_BP.ArbolNavidad_BP_C" :!class /Script/Engine.PrimitiveComponent)
    (Variables|Default|SetUnderTheTree? true)
    (Sprite|SetSpriteColor (Variables|Default|GetPresent_FB) "(R=1.000000,G=1.000000,B=1.000000,A=1.000000)")))

(event EventInteract
  (if (not (Variables|Default|GetUnderTheTree?))
    (Default|TakePresent (.AsFirst%20Person%20Character (Utilities|Casting|CastToFirstPersonCharacter (Game|Player|GetPlayerPawn 0))))
    (Actor|DestroyActor)))

(fn ConstructionScript)